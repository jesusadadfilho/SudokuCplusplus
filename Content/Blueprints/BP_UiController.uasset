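; BP_UiController switches the Sudoku game between the main menu and the board UI.
; On BeginPlay it creates the main menu widget, passing itself as a reference, and removes any existing game UI.
; SetupBoard swaps the menu for the main UI, then CreateRows pulls each row from the Sudoku controller and adds it to the board widget.
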(event `self.ReceiveBeginPlay`
  (`self.OpenMainMenu`))

(event `OpenMainMenu`
  (bind _wbp_mainui (`self.WBP_MainUi`))
  (bind _returnvalue (`|CreateWidget` "/Game/Blueprints/WIdget/WBP_MainMenu.WBP_MainMenu_C" null self))
  (bind _output_get (set `self.WBP_MainMenu` _returnvalue))
  (`UserWidget.AddToViewport` _output_get 0)
  (`/Engine/EditorBlueprintResources/StandardMacros.IsValid` _wbp_mainui
    (:`Is Valid`
      (`Widget.RemoveFromParent` _wbp_mainui))))

(event `SetupBoard`
  (`Widget.RemoveFromParent` (`self.WBP_MainMenu`))
  (bind _returnvalue (`|CreateWidget` "/Game/Blueprints/WIdget/WBP_MainUi.WBP_MainUi_C" null self))
  (set `self.WBP_MainUi` _returnvalue)
  (`UserWidget.AddToViewport` _returnvalue 0)
  (`self.CreateRows`))

(fn `CreateRows`
  (for _index (range (`SudokuController.CellSize` (`self.BP_SudokuController`)))
    (bind _returnvalue (`SudokuController.ReciveRowByIndex` (`self.BP_SudokuController`) _index))
    (`/Game/Blueprints/WIdget/WBP_Board.AddRow` (`/Game/Blueprints/WIdget/WBP_MainUi.WBP_Board` (`self.WBP_MainUi`)) _returnvalue)))

(fn `UserConstructionScript`)