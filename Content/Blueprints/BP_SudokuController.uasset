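; BP_SudokuController drives a Sudoku game's start-up and board setup.
; On BeginPlay it registers itself on the BP_PlayerPawn and shows the mouse cursor.
; Its BeginGame event runs in sequence: it sets up the puzzle from a base and difficulty, has the UI controller build the board, then starts play.
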(event `self.ReceiveBeginPlay`
  (bind _asbp_player_pawn (cast `/Game/Blueprints/BP_PlayerPawn` (`GameplayStatics.GetPlayerPawn` 0)))
  (set `/Game/Blueprints/BP_PlayerPawn.BP_SudokuController` self _asbp_player_pawn)
  (set `PlayerController.bShowMouseCursor` true (`GameplayStatics.GetPlayerController` 0)))

(event `BeginGame`
  (`|ExecutionSequence`
    (:`then_0`
      (`self.SetupSudoku` (`self.Sudoku Base`) (`self.Difficulty`)))
    (:`then_1`
      (`/Game/Blueprints/BP_UiController.SetupBoard` (`self.BP_UIController`)))
    (:`then_2`
      (`self.PlayGame`))))

(fn `UserConstructionScript`)